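; Content info subsystem Blueprint that adds MJ cost readouts to recipe tooltips and records research tree relationships between schematics.
; It hooks widget functions: cost slot PreConstruct injects an icon-text widget, and tooltip Construct fills it per ingredient and product with MJ and MJ-per-item-second values from GetRecipeCost.
; HandleResearchTreeSchematic finds a schematic's node, then adds schematics of nodes referencing its coordinates as parent, child or unhide links to its entry.
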(event `RecipeTooltip_Consttuct`
  (params (Object :type "Object Object Reference"))
  (bind _aswidget_tooltip_recipe (cast `/Game/FactoryGame/Interface/UI/InGame/Widget_TooltipRecipe` Object))
  (bind _mrecipe (`/Game/FactoryGame/Interface/UI/InGame/Widget_TooltipRecipe.mRecipe` _aswidget_tooltip_recipe))
  (if (`KismetSystemLibrary.IsValidClass` _mrecipe)
    (bind (_cost_total _amount _mjs_ingredient _productamount _mjs_products _ingredientmjis1 _producttmjsis1) (`/ContentInfo/BP_TooltipHelper.GetRecipeCost` _mrecipe))
    (for (_array_element _array_index) (`PanelWidget.GetAllChildren` (`/Game/FactoryGame/Interface/UI/InGame/Widget_TooltipRecipe.mIngredientsContainer` _aswidget_tooltip_recipe))
      (bind _aswidget_cost_slot_wrapper (cast `/Game/FactoryGame/Interface/UI/InGame/Widget_CostSlotWrapper` _array_element))
      (bind _asoverlay (cast `Overlay` (`Widget.GetParent` (`/Game/FactoryGame/Interface/UI/InGame/Widget_CostSlotWrapper.StackSizeOverlay` _aswidget_cost_slot_wrapper))))
      (for _array_element_2 (`PanelWidget.GetAllChildren` _asoverlay)
        (bind _aswidget_icon_text_icon (cast `/ContentInfo/Widget/TextLine/Widget_IconText_Icon` _array_element_2))
        (set `/ContentInfo/Widget/TextLine/Widget_IconText_Icon.IsRecipe` true _aswidget_icon_text_icon)
        (`/ContentInfo/Widget/TextLine/Widget_IconText_Icon.ReInit` _aswidget_icon_text_icon (`|GetArrayItem` _mjs_ingredient _array_index) (`|GetArrayItem` _ingredientmjis1 _array_index))
        (break)))
    (for (_array_element_3 _array_index_2) (`PanelWidget.GetAllChildren` (`/Game/FactoryGame/Interface/UI/InGame/Widget_TooltipRecipe.mProductsContainer` _aswidget_tooltip_recipe))
      (bind _aswidget_cost_slot_wrapper_2 (cast `/Game/FactoryGame/Interface/UI/InGame/Widget_CostSlotWrapper` _array_element_3))
      (bind _asoverlay_2 (cast `Overlay` (`Widget.GetParent` (`/Game/FactoryGame/Interface/UI/InGame/Widget_CostSlotWrapper.StackSizeOverlay` _aswidget_cost_slot_wrapper_2))))
      (for _array_element_4 (`PanelWidget.GetAllChildren` _asoverlay_2)
        (bind _aswidget_icon_text_icon_2 (cast `/ContentInfo/Widget/TextLine/Widget_IconText_Icon` _array_element_4))
        (set `/ContentInfo/Widget/TextLine/Widget_IconText_Icon.IsRecipe` true _aswidget_icon_text_icon_2)
        (`/ContentInfo/Widget/TextLine/Widget_IconText_Icon.ReInit` _aswidget_icon_text_icon_2 (`|GetArrayItem` _mjs_products _array_index_2) (`|GetArrayItem` _producttmjsis1 _array_index_2))
        (break)))))

(event `InitBindings`
  (`ContentInfoBPFuncLib.BindOnBPFunction` "/Game/FactoryGame/Interface/UI/InGame/Widget_TooltipRecipe.Widget_TooltipRecipe_C" (delegate `RecipeTooltip_Consttuct`) "Construct")
  (`ContentInfoBPFuncLib.BindOnBPFunction` "/Game/FactoryGame/Interface/UI/InGame/Widget_CostSlotWrapper.Widget_CostSlotWrapper_C" (delegate `CostSlotPreConstruct`) "PreConstruct"))

(event `CostSlotPreConstruct`
  (params (Object :type "Object Object Reference"))
  (bind _aswidget_cost_slot_wrapper (cast `/Game/FactoryGame/Interface/UI/InGame/Widget_CostSlotWrapper` Object))
  (bind _asoverlay (cast `Overlay` (`Widget.GetParent` (`/Game/FactoryGame/Interface/UI/InGame/Widget_CostSlotWrapper.StackSizeOverlay` _aswidget_cost_slot_wrapper))))
  (bind _returnvalue (`|CreateWidget` "/ContentInfo/Widget/TextLine/Widget_IconText_Icon.Widget_IconText_Icon_C" null 0.0 "HAlign_Left" false _aswidget_cost_slot_wrapper))
  (bind _returnvalue_2 (`Overlay.AddChildToOverlay` _asoverlay _returnvalue))
  (`OverlaySlot.SetVerticalAlignment` _returnvalue_2 "VAlign_Fill")
  (`OverlaySlot.SetHorizontalAlignment` _returnvalue_2 "HAlign_Fill"))

(fn `HandleResearchTreeSchematic`
  (params (Schematic :type "FGSchematic Class Reference") (Array :type "FGResearchTree Class Reference"))
  (returns (ReturnValue :type "Nogs_Schematic Structure"))
  (locals (Us :type "/Game/FactoryGame/Interface/UI/InGame/MAMTree/MAMTree_NodeData_Struct Structure") (Nodes :type "Array of FGResearchTreeNode Object Reference") (NewEntry :type "Nogs_Schematic Structure"))
  (bind _returnvalue (subsystem `/Game/BP_ContentInfoSubsystem`))
  (bind ((`Coordinates_23_5A3DE6C040C7026EDEA49E9CE8612292` _coordinates)) (break `/Game/FactoryGame/Interface/UI/InGame/MAMTree/MAMTree_NodeData_Struct` (`local.Us`)))
  (bind _returnvalue_2 (`FGResearchTree.GetNodes` Array))
  (set `local.Nodes` _returnvalue_2)
  (for _array_element (`local.Nodes`)
    (bind _asbpd_research_tree_node (cast `/Game/FactoryGame/Schematics/Research/BPD_ResearchTreeNode` _array_element))
    (bind _mnodedatastruct (`/Game/FactoryGame/Schematics/Research/BPD_ResearchTreeNode.mNodeDataStruct` _asbpd_research_tree_node))
    (bind ((`Schematic_27_3663A42446FDB4387D0C81AFC23E225B` _schematic)) (break `/Game/FactoryGame/Interface/UI/InGame/MAMTree/MAMTree_NodeData_Struct` _mnodedatastruct))
    (if (== Schematic _schematic)
      (set `local.Us` _mnodedatastruct)
      (bind _returnvalue_3 (`self.HandleSchematic` _returnvalue _schematic))
      (set `local.NewEntry` _returnvalue_3)
      (break)))
  (for _array_element_2 (`local.Nodes`)
    (bind _asbpd_research_tree_node_2 (cast `/Game/FactoryGame/Schematics/Research/BPD_ResearchTreeNode` _array_element_2))
    (bind ((`Schematic_27_3663A42446FDB4387D0C81AFC23E225B` _schematic_2) (`Parents_20_7A099B96409362536B743BA1CC77C234` _parents) (`ChildrenAndRoads_34_758C9E0D4F09DAF4BBAD309358952A0A` _childrenandroads) (`UnhiddenBy_38_909B07D7461225A33C48A68A7139FE63` _unhiddenby) (`NodesToUnhide_33_A6E465554D49C98EE2A0ECB493BE5CBA` _nodestounhide)) (break `/Game/FactoryGame/Interface/UI/InGame/MAMTree/MAMTree_NodeData_Struct` (`/Game/FactoryGame/Schematics/Research/BPD_ResearchTreeNode.mNodeDataStruct` _asbpd_research_tree_node_2)))
    (if (`KismetArrayLibrary.Array_Contains` _parents _coordinates)
      (`self.AddToSchematicArrayProp` (subsystem `ContentInfoSubsystem`) (`local.NewEntry`) _schematic_2 1))
    (if (`BlueprintMapLibrary.Map_Contains` _childrenandroads _coordinates)
      (`self.AddToSchematicArrayProp` _returnvalue (`local.NewEntry`) _schematic_2 2))
    (if (`KismetArrayLibrary.Array_Contains` _unhiddenby _coordinates)
      (`self.AddToSchematicArrayProp` _returnvalue (`local.NewEntry`) _schematic_2 2))
    (if (`KismetArrayLibrary.Array_Contains` _nodestounhide _coordinates)
      (`self.AddToSchematicArrayProp` _returnvalue (`local.NewEntry`) _schematic_2 3)))
  (return (`local.NewEntry`)))