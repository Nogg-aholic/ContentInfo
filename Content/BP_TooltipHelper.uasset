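; Helper functions for recipe tooltips that work out energy (MJ) values for Satisfactory ingredients and products.
; Ingredient and recipe MJ values come from the ContentInfo subsystem, with product costs adding the first producer's power use per cycle.
; Per-second functions also return readable formula strings, scaling non-solids by 1000.
; Formatters convert MJ to KJ–PJ units and build recipe lines with indexed texture placeholders.
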(fn `FormatRecipeTextLine`
  (params (TargetArray :type "Array of Texture2D Object Reference (by ref)") (Array :type "Array of Texture2D Object Reference") (Array1 :type "Array of Integer") (Array2 :type "Array of Float (double-precision)"))
  (returns (Line :type String))
  (locals (Strinh :type String))
  (bind _strinh (`local.Strinh`))
  (for (_array_element _array_index) Array
    (set `local.Strinh` (`KismetStringLibrary.Concat_StrStr` _strinh (`KismetMathLibrary.SelectString` "" "+" (`KismetStringLibrary.EqualEqual_StrStr` _strinh)) (`KismetStringLibrary.Concat_StrStr` (`KismetStringLibrary.Conv_IntToString` (`|GetArrayItem` Array1 _array_index)) "x" (`self.TextureToIndexString` _array_element TargetArray) "(" (`KismetTextLibrary.Conv_TextToString` (`KismetTextLibrary.Conv_DoubleToText` (`|GetArrayItem` Array2 _array_index) "HalfToEven" false true 1 324 0 1)) "MJ)"))))
  (return (`local.Strinh`)))

(fn `GetFirstBuildable`
  (params (Array :type "Array of Object Class Reference"))
  (returns (`AsFGBuildable Factory` :type "FGBuildableFactory Class Reference"))
  (for _array_element Array
    (bind _asfgbuildable_factory (castclass `FGBuildableFactory` _array_element))
    (return _asfgbuildable_factory)))

(fn `GetIngredientMJ`
  (params (ItemAmount :type "ItemAmount Structure (by ref)"))
  (returns (`MJ Total` :type "Float (double-precision)") (MJValue :type "Float (double-precision)"))
  (bind (_itemclass _amount) (break `ItemAmount` ItemAmount))
  (bind ((`ItemClass` _itemclass_2) (`MJValue` _mjvalue)) (break `Nogs_Descriptor` (`BlueprintMapLibrary.Map_Find` (`ContentInfoSubsystem.nItems` (subsystem `/ContentInfo/BP_ContentInfoSubsystem`)) _itemclass)))
  (return (* _amount _mjvalue) _mjvalue))

(fn `GetIngredientValues`
  (params (inClass :type "FGRecipe Class Reference") (Idx :type Integer))
  (returns (MJ :type "Float (double-precision)") (MJPerSec :type "Float (double-precision)") (String :type String))
  (bind _output (`|GetArrayItem` (`FGRecipe.GetIngredients` inClass) Idx))
  (bind (_itemclass _amount) (break `ItemAmount` _output))
  (bind (_mj_total _mjvalue) (`self.GetIngredientMJ` _output))
  (bind (_returnvalue _string) (`self.MJIPSecIngredient` (`FGRecipe.GetManufacturingDuration` inClass) _mjvalue _amount (`FGItemDescriptor.GetForm` _itemclass)))
  (return _mj_total _returnvalue _string))

(fn `GetProductMJValues`
  (params (inClass :type "FGRecipe Class Reference") (Idx :type Integer))
  (returns (MJ :type "Float (double-precision)") (MJPerSec :type "Float (double-precision)") (String :type String) (`BuidlingsFor 1 PerSec` :type "Float (double-precision)"))
  (bind (_ingredient_total_cost _cyclecost1 _totalcostfirstfactory) (`self.GetRecipeMJCost` inClass))
  (bind _returnvalue (`FGRecipe.GetManufacturingDuration` inClass))
  (bind (_itemclass _amount) (break `ItemAmount` (`|GetArrayItem` (`FGRecipe.GetProducts` inClass) Idx)))
  (bind (_returnvalue_2 _returnvalue1) (`self.MJPerSecProduct` _returnvalue _ingredient_total_cost (`FGItemDescriptor.GetForm` _itemclass) _amount (`KismetMathLibrary.FClamp` (- _totalcostfirstfactory _ingredient_total_cost) 0.0 34343333888.0)))
  (return (/ _totalcostfirstfactory (`KismetMathLibrary.Conv_IntToDouble` _amount)) _returnvalue_2 _returnvalue1 (`self.MachinesFor1PerSec` _returnvalue _amount)))

(fn `GetRecipeCost`
  (params (inClass :type "FGRecipe Class Reference"))
  (returns (`Cost Total` :type "Float (double-precision)") (`Ingredient Amounts` :type "Array of Integer") (`MJs Ingredient` :type "Array of Float (double-precision)") (ProductAmount :type "Array of Integer") (`MJs Products` :type "Array of Float (double-precision)") (`IngredientMJ per sec` :type "Array of Float (double-precision)") (`ProductMJ per sec` :type "Array of Float (double-precision)") (`Product MJ Per Sec Per Item` :type "Array of Float (double-precision)") (TTi1 :type "Array of String") (TTP1 :type "Array of String"))
  (locals (IngredientItemIcons :type "Array of Texture2D Object Reference") (IngredientAmounts :type "Array of Integer") (IngredientMJs :type "Array of Float (double-precision)") (CostTotal :type "Float (double-precision)") (ProductTextures :type "Array of Texture2D Object Reference") (ProductAmounts :type "Array of Integer") (ProducttMJs :type "Array of Float (double-precision)") (Buildable :type "FGBuildableFactory Class Reference") (Obj :type "Nogs_Recipe Structure") (ProducttMJsIS :type "Array of Float (double-precision)") (IngredientMJIS :type "Array of Float (double-precision)") (IngredientMJIS_0 :type "Array of Float (double-precision)") (TTi :type "Array of String") (TTP :type "Array of String"))
  (bind _returnvalue (`FGRecipe.GetManufacturingDuration` inClass))
  (bind _returnvalue_2 (`FGRecipe.GetManufacturingDuration` inClass))
  (bind _costtotal (`local.CostTotal`))
  (bind _returnvalue_3 (* _returnvalue (`FGBuildableFactory.GetProducingPowerConsumption` (cast `FGBuildableFactory` (`ContentInfoBPFuncLib.Conv_ClassToObject` (`local.Buildable`)) :!pure true))))
  (set `local.Buildable` (`self.GetFirstBuildable` (`FGRecipe.GetProducedIn` inClass)))
  (set `local.Obj` (`BlueprintMapLibrary.Map_Find` (`ContentInfoSubsystem.nRecipes` (subsystem `/ContentInfo/BP_ContentInfoSubsystem`)) inClass))
  (for _array_element (`FGRecipe.GetIngredients` inClass)
    (bind (_itemclass _amount) (break `ItemAmount` _array_element))
    (`KismetArrayLibrary.Array_Add` (`local.IngredientAmounts`) _amount)
    (bind (_productinrecipe _ingredientinrecipe _itemclass_2 _mjvalue) (break `Nogs_Descriptor` (`BlueprintMapLibrary.Map_Find` (`ContentInfoSubsystem.nItems` (subsystem `/ContentInfo/BP_ContentInfoSubsystem`)) _itemclass)))
    (bind _returnvalue_4 (* _amount _mjvalue))
    (`KismetArrayLibrary.Array_Add` (`local.IngredientMJs`) _returnvalue_4)
    (set `local.CostTotal` (+ _returnvalue_4 (`local.CostTotal`)))
    (bind (_returnvalue_5 _string) (`self.MJIPSecIngredient` _returnvalue _mjvalue _amount (`FGItemDescriptor.GetForm` _itemclass)))
    (`KismetArrayLibrary.Array_Add` (`local.IngredientMJIS`) _returnvalue_5)
    (`KismetArrayLibrary.Array_Add` (`local.TTi`) _string))
  (for _array_element_2 (`FGRecipe.GetProducts` inClass)
    (bind (_itemclass_3 _amount_2) (break `ItemAmount` _array_element_2))
    (`KismetArrayLibrary.Array_Add` (`local.ProductAmounts`) _amount_2)
    (bind (_returnvalue_6 _returnvalue1) (`self.MJPerSecProduct` _returnvalue_2 _costtotal (`FGItemDescriptor.GetForm` _itemclass_3) _amount_2 _returnvalue_3))
    (`KismetArrayLibrary.Array_Add` (`local.ProducttMJsIS`) _returnvalue_6)
    (`KismetArrayLibrary.Array_Add` (`local.ProducttMJs`) (+ _returnvalue_3 _costtotal))
    (`KismetArrayLibrary.Array_Add` (`local.IngredientMJIS_0`) (`self.MachinesFor1PerSec` _returnvalue_2 _amount_2))
    (`KismetArrayLibrary.Array_Add` (`local.TTP`) _returnvalue1))
  (return (`local.CostTotal`) (`local.IngredientAmounts`) (`local.IngredientMJs`) (`local.ProductAmounts`) (`local.ProducttMJs`) (`local.IngredientMJIS`) (`local.ProducttMJsIS`) (`local.IngredientMJIS_0`) (`local.TTi`) (`local.TTP`)))

(fn `GetRecipeMJCost`
  (params (inClass :type "FGRecipe Class Reference"))
  (returns (`Ingredient Total Cost` :type "Float (double-precision)") (CycleCost1 :type "Map of Object Class Reference to Float (double-precision)") (TotalCostFirstFactory :type "Float (double-precision)"))
  (locals (Cost :type "Float (double-precision)") (CycleCost :type "Map of Object Class Reference to Float (double-precision)") (TotalFistFactory :type "Float (double-precision)"))
  (set `local.Cost` (`.MJ_Average` (break `Nogs_RecipeMJ` (`.MJ` (break `Nogs_Recipe` (`BlueprintMapLibrary.Map_Find` (`ContentInfoSubsystem.nRecipes` (subsystem `/ContentInfo/BP_ContentInfoSubsystem`)) inClass))))))
  (for _array_element (`FGRecipe.GetProducedIn` inClass)
    (bind _asfgbuildable_factory (castclass `FGBuildableFactory` _array_element)
      (:`then`
        (bind _asfgbuildable_factory_2 (cast `FGBuildableFactory` (`ContentInfoBPFuncLib.Conv_ClassToObject` _asfgbuildable_factory))
          (:`then`
            (bind _returnvalue (* (`FGRecipe.GetManufacturingDuration` inClass) (`FGBuildableFactory.GetProducingPowerConsumption` _asfgbuildable_factory_2)))
            (`BlueprintMapLibrary.Map_Add` (`local.CycleCost`) _array_element _returnvalue))
          (:`CastFailed`
            (`BlueprintMapLibrary.Map_Add` (`local.CycleCost`) _array_element (`FGRecipe.GetManualManufacturingDuration` inClass) :!label _label))))
      (:`CastFailed`
        (goto _label)))
    (`/Engine/EditorBlueprintResources/StandardMacros.DoOnce` false
      (:`Completed`
        (set `local.TotalFistFactory` (+ _returnvalue (`local.Cost`))))))
  (return (`local.Cost`) (`local.CycleCost`) (`local.TotalFistFactory`)))

(fn `MachinesFor1PerSec`
  (params (`M Duration` :type "Float (double-precision)") (`Produced Amount` :type Integer))
  (returns (ReturnValue :type "Float (double-precision)"))
  (return (/ (select `bool` (> `M Duration` 1.0) :`false` (/ 1.0 `M Duration`) :`true` `M Duration`) (`KismetMathLibrary.Conv_IntToDouble` `Produced Amount`))))

(fn `MJ Conversion`
  (params (InputPin :type "Float (double-precision)"))
  (returns (ReturnValue :type String))
  (locals (D :type Integer))
  (if (< InputPin 5.0)
    (set `local.D` 0)
    (elif (> InputPin 1000.0)
      (set `local.D` 2)
      (if (> InputPin 1000000.0)
        (set `local.D` 3)
        (if (> InputPin 1000000000.0)
          (set `local.D` 4)))
      (else
        (set `local.D` 1))))
  (return (`KismetStringLibrary.Concat_StrStr` (`KismetTextLibrary.Conv_TextToString` (`KismetTextLibrary.Conv_DoubleToText` (/ InputPin (select `int` (`local.D`) :`0` 0.001 :`1` 1.0 :`2` 1000.0 :`3` 1000000.0 :`4` 1000000000.0 :!type "Float (single-precision)")) "HalfToEven" false true 1 8 0 1)) " " (select `int` (`local.D`) :`0` "KJ" :`1` "MJ" :`2` "GJ" :`3` "TJ" :`4` "PJ"))))

(fn `MJIPSecIngredient`
  (params (`Manufacturing Duration` :type "Float (double-precision)") (MJ :type "Float (double-precision)") (Amount :type Integer) (Form :type "EResourceForm Enum" :default "RF_INVALID"))
  (returns (ReturnValue :type "Float (double-precision)") (String :type String))
  (bind _returnvalue (`|EnumEquality` Form "RF_SOLID"))
  (bind _returnvalue_2 (* MJ (`KismetMathLibrary.Conv_IntToDouble` Amount)))
  (bind _returnvalue_3 (* (/ _returnvalue_2 `Manufacturing Duration`) (select `bool` _returnvalue :`false` 1000.0 :`true` 1.0 :!type "Float (single-precision)")))
  (return _returnvalue_3 (`KismetStringLibrary.Concat_StrStr` (`KismetStringLibrary.Concat_StrStr` "(" (`KismetStringLibrary.Conv_DoubleToString` MJ) "MJ)" "*" "(" (`KismetStringLibrary.Conv_IntToString` Amount) "items)" "= " (`KismetStringLibrary.Conv_DoubleToString` _returnvalue_2) "MJ Total") "/" (`KismetStringLibrary.Concat_StrStr` "(" (`KismetStringLibrary.Conv_DoubleToString` `Manufacturing Duration`) "sec)") (select `bool` _returnvalue :`false` "* 1000 ( Liquid ^3)") " = " (`KismetStringLibrary.Conv_DoubleToString` _returnvalue_3))))

(fn `MJPerSecProduct`
  (params (`Manufacturing Duration` :type "Float (double-precision)") (MJ :type "Float (double-precision)") (Form :type "EResourceForm Enum" :default "RF_INVALID") (Amount :type Integer) (`MJ Per Cycle` :type "Float (double-precision)"))
  (returns (ReturnValue :type "Float (double-precision)") (ReturnValue1 :type String))
  (bind _returnvalue (`|EnumEquality` Form "RF_SOLID"))
  (bind _returnvalue_2 (/ (* (+ MJ `MJ Per Cycle`) (select `bool` _returnvalue :`false` 1000.0 :`true` 1.0 :!type "Float (single-precision)")) `Manufacturing Duration`))
  (return _returnvalue_2 (`KismetStringLibrary.Concat_StrStr` (`KismetStringLibrary.Concat_StrStr` "(" (`KismetStringLibrary.Conv_DoubleToString` MJ) "MJ)" "+ (" (`KismetStringLibrary.Conv_DoubleToString` `MJ Per Cycle`) "MJ Per Cycle)" (select `bool` _returnvalue :`false` "* 1000 ( Liquid ^3)")) "/" (`KismetStringLibrary.Concat_StrStr` "(" (`KismetStringLibrary.Conv_DoubleToString` `Manufacturing Duration`) "sec)") " = " (`KismetStringLibrary.Conv_DoubleToString` _returnvalue_2))))

(fn `TextureToIndexString`
  (params (ItemToFind :type "Texture2D Object Reference (by ref)") (TargetArray :type "Array of Texture2D Object Reference (by ref)"))
  (returns (ReturnValue :type String))
  (if (`KismetArrayLibrary.Array_Contains` TargetArray ItemToFind)
    (return (`KismetStringLibrary.Concat_StrStr` "{" (`KismetStringLibrary.Conv_IntToString` (`KismetArrayLibrary.Array_Find` TargetArray ItemToFind)) "}"))
    (else
      (bind _returnvalue (`KismetArrayLibrary.Array_Add` TargetArray ItemToFind))
      (return (`KismetStringLibrary.Concat_StrStr` "{" (`KismetStringLibrary.Conv_IntToString` _returnvalue) "}")))))