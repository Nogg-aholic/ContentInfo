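; BP_ContentInfoInputHandler maps ContentInfo input actions to tooltip display controls on the BPContentInfoSubsystem.
; The TT and TTA actions call the subsystem's ShowTooltips and ShowTooltipsAdvanced functions on press.
; The TTH and TTHA actions work as holds, setting the normal and advanced tooltip overwrite flags while pressed and clearing them on release.
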(event `InputAction|ContentInfo.TT` :consume false :overrideparent false
  (params (Key :type "Key Structure"))
  (:`Pressed`
    (`/ContentInfo/BP_ContentInfoSubsystem.ShowTooltips` (subsystem `/ContentInfo/BP_ContentInfoSubsystem`))))

(event `InputAction|ContentInfo.TTA` :consume false :overrideparent false
  (params (Key :type "Key Structure"))
  (:`Pressed`
    (`/ContentInfo/BP_ContentInfoSubsystem.ShowTooltipsAdvanced` (subsystem `/ContentInfo/BP_ContentInfoSubsystem`))))

(event `InputAction|ContentInfo.TTH` :consume false :overrideparent false
  (params (Key :type "Key Structure"))
  (bind _returnvalue (subsystem `/ContentInfo/BP_ContentInfoSubsystem`))
  (:`Pressed`
    (set `/ContentInfo/BP_ContentInfoSubsystem.ShowTooltips_Overwrite` true _returnvalue))
  (:`Released`
    (set `/ContentInfo/BP_ContentInfoSubsystem.ShowTooltips_Overwrite` false _returnvalue)))

(event `InputAction|ContentInfo.TTHA` :consume false :overrideparent false
  (params (Key :type "Key Structure"))
  (bind _returnvalue (subsystem `/ContentInfo/BP_ContentInfoSubsystem`))
  (:`Pressed`
    (set `/ContentInfo/BP_ContentInfoSubsystem.ShowTooltips_Overwrite_Adv` true _returnvalue))
  (:`Released`
    (set `/ContentInfo/BP_ContentInfoSubsystem.ShowTooltips_Overwrite_Adv` false _returnvalue)))

(fn `UserConstructionScript`)